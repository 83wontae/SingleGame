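; BP_SingleHUD is a single-mode HUD Blueprint that creates the SingleHudWidget on BeginPlay and adds it to the viewport.
; It exposes wrapper functions that cast the stored widget and forward calls to position or hide a pickup guide and show the death UI.
; BeginPlay also starts a fast looping timer targeting UpdateCountDown by name, though no such function appears in this Blueprint's graphs.
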(event `self.ReceiveBeginPlay`
  (bind _returnvalue (`|CreateWidget` "/Game/FirstGame/Widget/SingleHudWidget.SingleHudWidget_C"))
  (bind _output_get (set `self.HudWidget` _returnvalue))
  (`UserWidget.AddToViewport` _output_get 0)
  (`KismetSystemLibrary.K2_SetTimer` null "UpdateCountDown" 0.01 true))

(fn `HidePickUpGuide`
  (bind _assingle_hud_widget (cast `/Game/FirstGame/Widget/SingleHudWidget` (`self.HudWidget`)))
  (`/Game/FirstGame/Widget/SingleHudWidget.HideGuidePostion` _assingle_hud_widget))

(fn `ShowDeathUI`
  (bind _assingle_hud_widget (cast `/Game/FirstGame/Widget/SingleHudWidget` (`self.HudWidget`)))
  (`/Game/FirstGame/Widget/SingleHudWidget.ShowDeathUI` _assingle_hud_widget true))

(fn `UpdatePickUpGuidePosition`
  (params (WorldLocation :type "Vector Structure"))
  (bind _assingle_hud_widget (cast `/Game/FirstGame/Widget/SingleHudWidget` (`self.HudWidget`)))
  (`/Game/FirstGame/Widget/SingleHudWidget.UpdateGuidePostion` _assingle_hud_widget WorldLocation))

(fn `UserConstructionScript`
  (`parent.UserConstructionScript`))