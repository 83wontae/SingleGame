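; BP_EscalatorFloor is a moving escalator step actor that travels repeatedly along a spline.
; A looping timer advances its distance by Speed and sets the actor to the spline's world transform at that point.
; Past the spline's end, it hides the cube and disables its collision, then after a short delay teleports back to the start, restores both and restarts the movement timer.
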(event `self.ReceiveBeginPlay`
  (`KismetSystemLibrary.K2_SetTimer` null "UpdateMoveFloor" 0.01 true))

(fn `SetStartPoint`
  (bind _cube (`self.Cube`))
  (bind _output_get (set `self.Distance` 0.0))
  (`self.K2_SetActorTransform` (`SplineComponent.GetTransformAtDistanceAlongSpline` (`self.Spline`) _output_get "World" false) false true)
  (`SceneComponent.SetVisibility` _cube true false)
  (`PrimitiveComponent.SetCollisionEnabled` _cube "QueryAndPhysics")
  (`KismetSystemLibrary.K2_SetTimer` null "UpdateMoveFloor" 0.01 true))

(fn `UpdateMoveFloor`
  (bind _cube (`self.Cube`))
  (bind _output_get (set `self.Distance` (+ (* 0.01 (`self.Speed`)) (`self.Distance`))))
  (`self.K2_SetActorTransform` (`SplineComponent.GetTransformAtDistanceAlongSpline` (`self.Spline`) _output_get "World" false))
  (if (> (`self.Distance`) (`SplineComponent.GetSplineLength` (`self.Spline`)))
    (`SceneComponent.SetVisibility` _cube false false)
    (`PrimitiveComponent.SetCollisionEnabled` _cube "NoCollision")
    (`KismetSystemLibrary.K2_SetTimer` null "SetStartPoint" 0.1)
    (`KismetSystemLibrary.K2_ClearTimer` null "UpdateMoveFloor")))

(fn `UserConstructionScript`)